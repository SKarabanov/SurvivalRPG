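; Game mode for the start menu that shows the main menu and load window widgets.
; On BeginPlay in L_StartMenu it polls every 0.1 seconds until the player controller is valid, then opens the main menu.
; ShowMainMenu and ShowLoadMenu each create their widget once, cache it and add it to the viewport.
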(event Custom|ShowLoadMenu
  ;[1 1 1] Show Load Menu
  (Utilities|IsValid (Variables|Default|GetW_Load)
    (:Is%20Valid
      _)
    (:Is%20Not%20Valid
      (bind _returnvalue (UserInterface|CreateWidget "/Game/Project/Widgets/W_LoadWindow.W_LoadWindow_C"))
      (Variables|Default|SetW_Load _returnvalue)))
  (UserInterface|Viewport|AddtoViewport (Variables|Default|GetW_Load) 0))

(event Custom|ShowMainMenu
  ;[1 1 1] Show Main menu
  (Utilities|IsValid (Variables|Default|GetMainMenu)
    (:Is%20Valid
      _)
    (:Is%20Not%20Valid
      (bind _returnvalue (UserInterface|CreateWidget "/Game/Project/Widgets/W_StartMenu.W_StartMenu_C" (Game|GetPlayerController 0)))
      (Variables|Default|SetMainMenu _returnvalue)))
  (UserInterface|Viewport|AddtoViewport (Variables|Default|GetMainMenu) 0))

(event EventBeginPlay
  (bind _returnvalue (Game|GetCurrentLevelName true))
  (if (Utilities|Enum|Equal(Enum) _returnvalue "L_StartMenu")
    (Utilities|IsValid (Game|GetPlayerController 0) :!label _label
      (:Is%20Valid
        (CallFunction|ShowMainMenu))
      (:Is%20Not%20Valid
        (Utilities|FlowControl|Delay 0.1)
        (goto _label)))))

(fn ConstructionScript)