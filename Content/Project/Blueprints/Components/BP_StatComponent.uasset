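; BP_StatComponent is an actor component that tracks a character's health and shows it as floating text.
; SRV_ChangeHealth adds a signed amount to HPCurrent and clamps it between zero and HPMAX.
; HPCurrent's RepNotify writes the value to the owning ThirdPersonCharacter's TextRender, only where the owner lacks authority, so the server's text is not updated here.
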(event Custom|SRV_ChangeHealth
  (params (Add :type Float%20%28single-precision%29))
  (Variables|Default|SetHP_Current (Math|Float|Clamp(Float) (+ Add (Variables|Default|GetHP_Current)) 0.0 (Variables|Default|GetHP_MAX))))

(fn OnRepHPCurrent
  (if (not (Ability|HasAuthority (Components|GetOwner)))
    (bind _asthird_person_character (Utilities|Casting|CastToThirdPersonCharacter (Components|GetOwner)))
    (Rendering|Components|TextRender|SetText (Variables|/Game/ThirdPersonBP/Blueprints/ThirdPersonCharacter.ThirdPersonCharacter_C|GetTextRender _asthird_person_character) (Utilities|Text|ToText(Float) (Variables|Default|GetHP_Current) "HalfToEven"))))